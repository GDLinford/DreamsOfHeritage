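; An interactable actor that changes a screen's material and plays music when the player presses E nearby.
; Begin and end overlap on a box component set a flag without filtering the overlapping actor.
; Tick checks that flag and polls the E key on the first player controller, then sets the Screen's first material slot and starts Music from the beginning.
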(event OnComponentBeginOverlap(Box)
  (params (OverlappedComponent :type Primitive%20Component%20Object%20Reference) (OtherActor :type Actor%20Object%20Reference) (OtherComp :type Primitive%20Component%20Object%20Reference) (OtherBodyIndex :type Integer) (bFromSweep :type Boolean) (SweepResult :type Hit%20Result%20Structure%20%28by%20ref%29))
  (Variables|Default|SetOverlapChangeMat true))

(event OnComponentEndOverlap(Box)
  (params (OverlappedComponent :type Primitive%20Component%20Object%20Reference) (OtherActor :type Actor%20Object%20Reference) (OtherComp :type Primitive%20Component%20Object%20Reference) (OtherBodyIndex :type Integer))
  (Variables|Default|SetOverlapChangeMat false))

(event EventTick
  (params (DeltaSeconds :type Float%20%28single-precision%29))
  (Utilities|Casting|CastToFirstPersonCharacter (Game|GetPlayerCharacter 0))
  (if (Variables|Default|GetOverlapChangeMat)
    (if (Game|Player|WasInputKeyJustPressed (Game|GetPlayerController 0) "E")
      (Rendering|Material|SetMaterial (Variables|Default|GetScreen) 0 (Variables|Default|GetMaterial))
      (Audio|Components|Audio|Play (Variables|Default|GetMusic) 0.0))))

(fn ConstructionScript)